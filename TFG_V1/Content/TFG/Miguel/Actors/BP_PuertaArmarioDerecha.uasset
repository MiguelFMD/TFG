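; BP_PuertaArmarioDerecha is the right-hand door of a wardrobe, which swings open or closed each time its AbrirPuertaDerecha event fires.
; The Closed flag selects the Open or Close timeline, whose track sets the actor's absolute world yaw while keeping its pitch and roll.
; A Moving flag ignores new calls until the timeline finishes and a short delay passes.
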(event Custom|AbrirPuertaDerecha
  (bind _returnvalue (Transformation|GetActorRotation))
  (bind _returnvalue_2 (Transformation|GetActorRotation))
  (if (not (Variables|Default|GetMoving))
    (Variables|Default|SetMoving true)
    (if (Variables|Default|GetClosed)
      (Variables|Default|SetClosed false)
      (bind _newtrack_0 (Timeline|Open PlayFromStart)
        (:Update
          (Transformation|SetActorRotation (Math|Rotator|MakeRotator (.roll _returnvalue_2) (.pitch _returnvalue_2) _newtrack_0)))
        (:Finished
          (Utilities|FlowControl|Delay 0.2)
          (Variables|Default|SetMoving false)))
      (else
        (Variables|Default|SetClosed true)
        (bind _newtrack_0_2 (Timeline|Close PlayFromStart)
          (:Update
            (Transformation|SetActorRotation (Math|Rotator|MakeRotator (.roll _returnvalue) (.pitch _returnvalue) _newtrack_0_2)))
          (:Finished
            (Utilities|FlowControl|Delay 0.2)
            (Variables|Default|SetMoving false)))))))

(fn ConstructionScript
  (|CallParentFunction))