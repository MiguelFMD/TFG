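; BP_KeyObject is an interaction dispatcher that routes a BeginInteract event to the behavior matching the target actor's class.
; Chained class checks send BP_CheckObject targets to BeginCheck, passing the actor along, and BP_Shortcut targets to BeginShortCut.
; Any other actor falls through an always-true branch, is cast to BP_HidingPlace and told to Hide, with no class check.
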(event Custom|BeginInteract
  (params (InteractActor :type Actor%20Object%20Reference))
  (if (Utilities|ClassIsChildOf (Utilities|GetClass InteractActor) "/Game/TFG/Miguel/Actors/BP_CheckObject.BP_CheckObject_C")
    (Default|BeginCheck (.AsBP%20Check%20Object (Utilities|Casting|CastToBP_CheckObject InteractActor)) InteractActor)
    (elif (Utilities|ClassIsChildOf (Utilities|GetClass InteractActor) "/Game/TFG/Miguel/Actors/BP_Shortcut.BP_Shortcut_C")
      (Default|BeginShortCut (.AsBP%20Shortcut (Utilities|Casting|CastToBP_Shortcut InteractActor)))
      (elif true
        (Default|Hide (.AsBP%20Hiding%20Place (Utilities|Casting|CastToBP_HidingPlace InteractActor)))))))

(fn ConstructionScript)