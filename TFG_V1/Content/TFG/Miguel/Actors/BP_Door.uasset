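; BP_Door is an interactable door that swings open and closed, optionally locked by a DoorID the player must hold.
; OpenDoor searches the FirstPersonCharacter's Keys for that ID, or skips the check when it is "None", then calls RotateDoor.
; RotateDoor plays or reverses a timeline driving mesh yaw, disabling interaction and custom-depth rendering until it finishes.
; Tick derives ClosedDoor from the timeline's Alpha to choose the direction.
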(event Custom|OpenDoor
  (params (Actor :type Actor%20Object%20Reference))
  (if (Utilities|Name|NotEqual(Name) (Variables|Default|GetDoorID) "None")
    (bind _asfirst_person_character (Utilities|Casting|CastToFirstPersonCharacter (Game|GetPlayerCharacter 0)))
    (bind _array_element (Utilities|Array|ForEachLoopwithBreak (Variables|/Game/Assets/FirstPersonBP/Blueprints/FirstPersonCharacter.FirstPersonCharacter_C|GetKeys _asfirst_person_character) :!label _label)
      (:LoopBody
        (if (Utilities|Name|Equal(Name) _array_element (Variables|Default|GetDoorID))
          (CallFunction|RotateDoor :!label _label_2)
          (goto _label Break))))
    (else
      (goto _label_2))))

(event Custom|RotateDoor
  (Variables|Default|SetInteractable false)
  (Rendering|SetRenderCustomDepth (Variables|Character|GetMesh) false)
  (if (Variables|Default|GetClosedDoor)
    (bind _alpha (Timeline|Rotate PlayFromStart)
      (:Update
        (Transformation|SetRelativeRotation (Variables|Character|GetMesh) (Math|Rotator|MakeRotator 0.0 0.0 _alpha) false false))
      (:Finished
        (Variables|Default|SetInteractable true)
        (Rendering|SetRenderCustomDepth (Variables|Character|GetMesh) true)))
    (else
      (Timeline|Rotate Reverse))))

(event EventTick
  (params (DeltaSeconds :type Float%20%28single-precision%29))
  (Variables|Default|SetClosedDoor (< (stale Custom|RotateDoor _alpha) 1.0)))

(fn ConstructionScript
  (|CallParentFunction))