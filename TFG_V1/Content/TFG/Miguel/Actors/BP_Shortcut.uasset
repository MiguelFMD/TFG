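; Shortcut actor that teleports the first-person player to its End component behind a screen fade.
; BeginShortCut disables player input and removes the game mode HUD's message widget, then plays a fade-to-black timeline on the player HUD.
; Location and control rotation snap to End on every fade-in update rather than once at full black.
; A second timeline then fades back in and restores input.
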(event Custom|BeginShortCut
  (params (Shortcut :type Actor%20Object%20Reference))
  (bind _returnvalue (Game|GetPlayerCharacter 0))
  (bind _returnvalue_2 (Game|GetPlayerCharacter 0))
  (bind _end (Variables|Default|GetEnd))
  (Input|DisableInput _returnvalue (Game|GetPlayerController 0))
  (bind _asfirst_person_character (Utilities|Casting|CastToFirstPersonCharacter _returnvalue))
  (Variables|/Game/Assets/FirstPersonBP/Blueprints/FirstPersonCharacter.FirstPersonCharacter_C|SetPlayerInput _asfirst_person_character false)
  (Widget|RemovefromParent (Variables|/Game/TFG/Miguel/UserInterface/HeadsUpDisplay.HeadsUpDisplay_C|GetMessageWidget (Variables|/Game/Assets/FirstPersonBP/Blueprints/FirstPersonGameMode.FirstPersonGameMode_C|GetHeadsUpDisplay (.AsFirst%20Person%20Game%20Mode (Utilities|Casting|CastToFirstPersonGameMode (Game|GetGameMode))))))
  (bind _newtrack_0 (Timeline|FadeIn PlayFromStart)
    (:Update
      (Class|Border|SetBrushColor (Variables|/Game/TFG/Miguel/UserInterface/HeadsUpDisplay.HeadsUpDisplay_C|GetFade (Variables|/Game/Assets/FirstPersonBP/Blueprints/FirstPersonCharacter.FirstPersonCharacter_C|GetPlayerHUD (.AsFirst%20Person%20Character (Utilities|Casting|CastToFirstPersonCharacter (Game|GetPlayerCharacter 0))))) (Math|Color|Lerp(LinearColor) "(R=0.000000,G=0.000000,B=0.000000,A=0.000000)" "(R=0.000000,G=0.000000,B=0.000000,A=1.000000)" _newtrack_0))
      (Transformation|SetActorLocation (Game|GetPlayerCharacter 0) (Transformation|GetWorldLocation _end) false true)
      (Pawn|SetControlRotation (Game|GetPlayerController 0) (Transformation|GetWorldRotation _end)))
    (:Finished
      (bind _newtrack_0_2 (Timeline|FadeOut PlayFromStart)
        (:Update
          (Class|Border|SetBrushColor (Variables|/Game/TFG/Miguel/UserInterface/HeadsUpDisplay.HeadsUpDisplay_C|GetFade (Variables|/Game/Assets/FirstPersonBP/Blueprints/FirstPersonCharacter.FirstPersonCharacter_C|GetPlayerHUD (.AsFirst%20Person%20Character (Utilities|Casting|CastToFirstPersonCharacter (Game|GetPlayerCharacter 0))))) (Math|Color|Lerp(LinearColor) :B "(R=0.000000,G=0.000000,B=0.000000,A=0.000000)" :Alpha _newtrack_0_2)))
        (:Finished
          (Input|EnableInput _returnvalue_2 (Game|GetPlayerController 0))
          (bind _asfirst_person_character_2 (Utilities|Casting|CastToFirstPersonCharacter _returnvalue_2))
          (Variables|/Game/Assets/FirstPersonBP/Blueprints/FirstPersonCharacter.FirstPersonCharacter_C|SetPlayerInput _asfirst_person_character_2 true))))))

(fn ConstructionScript
  (|CallParentFunction))