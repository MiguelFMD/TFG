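; BP_InteractableObject is an interactable actor, apparently a base for the game's usable objects, that routes player interactions to type-specific actions.
; It sets its Interactable flag on BeginPlay, and BeginInteract checks that flag on the passed actor.
; A chain of nested casts then calls the matching action for check objects, shortcuts, hiding places, keys, doors, drawers, or left and right wardrobe doors.
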(event Custom|BeginInteract
  (params (InteractActor :type Actor%20Object%20Reference))
  (bind (_asbp_hiding_place _bsuccess) (Utilities|Casting|CastToBP_HidingPlace InteractActor))
  (bind (_asbp_key _bsuccess_2) (Utilities|Casting|CastToBP_Key InteractActor))
  (bind (_asbp_puerta_armario_izquierda _bsuccess_3) (Utilities|Casting|CastToBP_PuertaArmarioIzquierda InteractActor))
  (bind (_asbp_door _bsuccess_4) (Utilities|Casting|CastToBP_Door InteractActor))
  (bind (_asbp_cajon _bsuccess_5) (Utilities|Casting|CastToBP_Cajon InteractActor))
  (bind (_asbp_puerta_armario_derecha _bsuccess_6) (Utilities|Casting|CastToBP_PuertaArmarioDerecha InteractActor))
  (bind (_asbp_check_object _bsuccess_7) (Utilities|Casting|CastToBP_CheckObject InteractActor))
  (bind (_asbp_shortcut _bsuccess_8) (Utilities|Casting|CastToBP_Shortcut InteractActor))
  (if (Variables|BP_InteractableObject_C|GetInteractable (.AsBP%20Interactable%20Object (Utilities|Casting|CastToBP_InteractableObject InteractActor)))
    (if _bsuccess_7
      (Default|BeginCheck _asbp_check_object InteractActor)
      (elif _bsuccess_8
        (Default|BeginShortCut _asbp_shortcut)
        (elif _bsuccess
          (Default|Hide _asbp_hiding_place)
          (elif _bsuccess_2
            (Default|CollectKey _asbp_key _asbp_key)
            (elif _bsuccess_4
              (Default|OpenDoor _asbp_door _asbp_door)
              (elif _bsuccess_5
                (Default|OpenDrawer _asbp_cajon _asbp_cajon)
                (elif _bsuccess_6
                  (Default|AbrirPuertaDerecha _asbp_puerta_armario_derecha)
                  (elif _bsuccess_3
                    (Default|AbrirPuertaIzquierda _asbp_puerta_armario_izquierda)))))))))))

(event EventBeginPlay
  (Variables|Default|SetInteractable true))

(fn ConstructionScript)