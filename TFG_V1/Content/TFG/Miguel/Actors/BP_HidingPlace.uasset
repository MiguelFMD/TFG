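; BP_HidingPlace is a hiding spot actor that lets the player hide inside it and climb back out.
; Hide flags the character as hidden, turns off its PlayerInput flag, clears the HUD message, teleports it to the HidingPlace component and shows an overlay widget.
; While hidden, Tick polls raw key presses against the FinishInteract action mapping, then teleports the player to the Mesh transform, restores input and removes the overlay.
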(event Custom|Hide
  (bind _returnvalue (Game|GetPlayerCharacter 0))
  (bind _hidingplace (Variables|Default|GetHidingPlace))
  (bind _asfirst_person_character (Utilities|Casting|CastToFirstPersonCharacter _returnvalue))
  (Variables|/Game/Assets/FirstPersonBP/Blueprints/FirstPersonCharacter.FirstPersonCharacter_C|SetPlayerInput _asfirst_person_character false)
  (Variables|/Game/Assets/FirstPersonBP/Blueprints/FirstPersonCharacter.FirstPersonCharacter_C|SetHiden _asfirst_person_character true)
  (Widget|RemovefromParent (Variables|/Game/TFG/Miguel/UserInterface/HeadsUpDisplay.HeadsUpDisplay_C|GetMessageWidget (Variables|/Game/Assets/FirstPersonBP/Blueprints/FirstPersonGameMode.FirstPersonGameMode_C|GetHeadsUpDisplay (.AsFirst%20Person%20Game%20Mode (Utilities|Casting|CastToFirstPersonGameMode (Game|GetGameMode))))))
  (Transformation|SetActorLocationAndRotation (Game|GetPlayerCharacter 0) (Transformation|GetWorldLocation _hidingplace) (Transformation|GetWorldRotation _hidingplace) false true)
  (bind _returnvalue_2 (UserInterface|CreateWidget "/Game/TFG/Miguel/UserInterface/HideInterface.HideInterface_C"))
  (bind _output_get (Variables|Default|SetHiding%20Interface _returnvalue_2))
  (UserInterface|Viewport|AddtoViewport _output_get 0))

(event EventTick
  (params (DeltaSeconds :type Float%20%28single-precision%29))
  (bind _returnvalue (Game|GetPlayerController 0))
  (bind _returnvalue_2 (Game|GetPlayerCharacter 0))
  (bind _hiding_interface (Variables|Default|GetHiding%20Interface))
  (bind _mesh (Variables|Character|GetMesh))
  (bind _asfirst_person_character (Utilities|Casting|CastToFirstPersonCharacter _returnvalue_2))
  (bind _asfirst_person_character_2 (Utilities|Casting|CastToFirstPersonCharacter (Game|GetPlayerCharacter 0)))
  (if (Variables|/Game/Assets/FirstPersonBP/Blueprints/FirstPersonCharacter.FirstPersonCharacter_C|GetHiden _asfirst_person_character_2)
    (if (Game|Player|WasInputKeyJustPressed (Game|GetPlayerController 0) "AnyKey")
      (for _array_element (Class|InputSettings|GetActionMappingbyName (Class|InputSettings|GetInputSettings) "FinishInteract")
        (if (Game|Player|WasInputKeyJustPressed (Game|GetPlayerController 0) (.Key (Utilities|Struct|BreakInputActionKeyMapping _array_element)))
          (Transformation|SetActorLocationAndRotation (Game|GetPlayerCharacter 0) (Transformation|GetWorldLocation _mesh) (Transformation|GetWorldRotation _mesh) false true)
          (Input|SetInputModeGameOnly _returnvalue)
          (Input|EnableInput _returnvalue_2 _returnvalue)
          (Variables|/Game/Assets/FirstPersonBP/Blueprints/FirstPersonCharacter.FirstPersonCharacter_C|SetPlayerInput _asfirst_person_character true)
          (Variables|/Game/Assets/FirstPersonBP/Blueprints/FirstPersonCharacter.FirstPersonCharacter_C|SetHiden _asfirst_person_character false)
          (Utilities|IsValid _hiding_interface
            (:Is%20Valid
              (Widget|RemovefromParent _hiding_interface))))))))

(fn ConstructionScript
  (|CallParentFunction))