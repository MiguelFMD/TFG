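; BP_Cajon is a drawer actor that slides open when its OpenDrawer event fires.
; The event sets a target DistanceMove along the actor's forward vector, clears Interactable and turns off the mesh's custom depth rendering.
; A timeline track then lerps the actor from its current location to that target.
; The file has no closing logic and never re-enables interaction.
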(event Custom|OpenDrawer
  (params (Actor :type Actor%20Object%20Reference))
  (bind _returnvalue (Transformation|GetActorLocation))
  (Variables|Default|SetTargetPoint (+ _returnvalue (* (Transformation|GetActorForwardVector) (Variables|Default|GetDistanceMove))))
  (Variables|Default|SetCurrentLocation _returnvalue)
  (Variables|Default|SetInteractable false)
  (Rendering|SetRenderCustomDepth (Variables|Character|GetMesh) false)
  (bind _newtrack_0 (Timeline|Timeline Play)
    (:Update
      (Transformation|SetActorLocation (Math|Vector|Lerp(Vector) (Variables|Default|GetCurrentLocation) (Variables|Default|GetTargetPoint) _newtrack_0) false false))))

(fn ConstructionScript
  (|CallParentFunction))