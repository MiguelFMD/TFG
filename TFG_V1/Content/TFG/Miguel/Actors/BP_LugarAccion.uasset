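; BP_LugarAccion is an action spot actor that pulls an IA_Loco character into place when it overlaps the spot's Box.
; On overlap it disables that character's capsule collision and plays the TeleportSmooth timeline from the start.
; Each update lerps the character's current location and rotation toward the Box's world transform by the timeline's Alpha, snapping it smoothly into position.
; Collision is not restored here.
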(event OnComponentBeginOverlap(Box)
  (params (OverlappedComponent :type Primitive%20Component%20Object%20Reference) (OtherActor :type Actor%20Object%20Reference) (OtherComp :type Primitive%20Component%20Object%20Reference) (OtherBodyIndex :type Integer) (bFromSweep :type Boolean) (SweepResult :type Hit%20Result%20Structure%20%28by%20ref%29))
  (bind _box (Variables|Default|GetBox))
  (bind _asia_loco (Utilities|Casting|CastToIA_Loco OtherActor))
  (Collision|SetCollisionEnabled (Variables|/Script/Engine.Character|GetCapsuleComponent _asia_loco) "NoCollision")
  (bind _alpha (Timeline|TeleportSmooth PlayFromStart)
    (:Update
      (Transformation|SetActorLocationAndRotation _asia_loco (Math|Vector|Lerp(Vector) (Transformation|GetActorLocation _asia_loco) (Transformation|GetWorldLocation _box) _alpha) (Math|Rotator|Lerp(Rotator) (Transformation|GetActorRotation _asia_loco) (Transformation|GetWorldRotation _box) _alpha)))))

(fn ConstructionScript)