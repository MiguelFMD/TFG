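; BP_KeyObject is an inspectable key object that the player examines up close in first person.
; BeginInteract blocks player input, enables mesh physics, moves the mesh to the character's VisualBox and swaps the HUD message for an ObjectInterface widget.
; While inspecting, Tick rotates the mesh by mouse delta and polls keys mapped to FinishInteract.
; Finishing returns the mesh to its BeginPlay transform, disables physics, restores input and removes the widget.
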(event Custom|BeginInteract
  (params (InteractActor :type Actor%20Object%20Reference))
  (bind _returnvalue (Game|GetPlayerCharacter 0))
  (bind _asbp_key_object (Utilities|Casting|CastToBP_KeyObject InteractActor))
  (bind _asfirst_person_character (Utilities|Casting|CastToFirstPersonCharacter _returnvalue))
  (bind _mesh (Variables|BP_KeyObject_C|GetMesh _asbp_key_object))
  (Variables|/Game/Assets/FirstPersonBP/Blueprints/FirstPersonCharacter.FirstPersonCharacter_C|SetPlayerInput _asfirst_person_character false)
  (Variables|Default|SetInteract%20Actor InteractActor)
  (Physics|SetSimulatePhysics _mesh true)
  (Components|MoveComponentTo _mesh (Transformation|GetWorldLocation (Variables|/Game/Assets/FirstPersonBP/Blueprints/FirstPersonCharacter.FirstPersonCharacter_C|GetVisualBox _asfirst_person_character)) "0, 0, 0" false false 0.2 false)
  (Widget|RemovefromParent (Variables|/Game/TFG/Miguel/UserInterface/HeadsUpDisplay.HeadsUpDisplay_C|GetMessageWidget (Variables|/Game/Assets/FirstPersonBP/Blueprints/FirstPersonGameMode.FirstPersonGameMode_C|GetHeadsUpDisplay (.AsFirst%20Person%20Game%20Mode (Utilities|Casting|CastToFirstPersonGameMode (Game|GetGameMode))))))
  (bind _returnvalue_2 (UserInterface|CreateWidget "/Game/TFG/Miguel/UserInterface/ObjectInterface.ObjectInterface_C"))
  (bind _output_get (Variables|Default|SetObjectInterface _returnvalue_2))
  (UserInterface|Viewport|AddtoViewport _output_get 0))

(event EventTick
  (params (DeltaSeconds :type Float%20%28single-precision%29))
  (bind _returnvalue (Game|GetPlayerController 0))
  (bind _returnvalue_2 (Game|GetPlayerCharacter 0))
  (bind _returnvalue_3 (Game|GetPlayerController 0))
  (bind _objectinterface (Variables|Default|GetObjectInterface))
  (bind (_deltax _deltay) (Class|PlayerController|GetInputMouseDelta _returnvalue_3))
  (if (not (Variables|/Game/Assets/FirstPersonBP/Blueprints/FirstPersonCharacter.FirstPersonCharacter_C|GetPlayerInput (.AsFirst%20Person%20Character (Utilities|Casting|CastToFirstPersonCharacter (Game|GetPlayerCharacter 0)))))
    (Utilities|IsValid (Variables|Default|GetInteract%20Actor)
      (:Is%20Valid
        (if (Game|Player|WasInputKeyJustPressed (Game|GetPlayerController 0) "AnyKey")
          (for _array_element (Class|InputSettings|GetActionMappingbyName (Class|InputSettings|GetInputSettings) "FinishInteract")
            (if (Game|Player|WasInputKeyJustPressed (Game|GetPlayerController 0) (.Key (Utilities|Struct|BreakInputActionKeyMapping _array_element)))
              (Components|MoveComponentTo (Variables|BP_KeyObject_C|GetMesh (.AsBP%20Key%20Object (Utilities|Casting|CastToBP_KeyObject (Variables|Default|GetInteract%20Actor)))) (Variables|Default|GetOriginalPosition) (Variables|Default|GetOriginalRotation) false false 0.2 false)
              (Physics|SetSimulatePhysics (Variables|BP_KeyObject_C|GetMesh (.AsBP%20Key%20Object (Utilities|Casting|CastToBP_KeyObject (Variables|Default|GetInteract%20Actor)))) false)
              (Input|SetInputModeGameOnly _returnvalue)
              (Input|EnableInput _returnvalue_2 _returnvalue)
              (Variables|/Game/Assets/FirstPersonBP/Blueprints/FirstPersonCharacter.FirstPersonCharacter_C|SetPlayerInput (.AsFirst%20Person%20Character (Utilities|Casting|CastToFirstPersonCharacter _returnvalue_2)) true)
              (Utilities|IsValid _objectinterface
                (:Is%20Valid
                  (Widget|RemovefromParent _objectinterface)
                  (Variables|Default|SetInteract%20Actor 0)))))
          (else
            (Transformation|AddLocalRotation (Variables|BP_KeyObject_C|GetMesh (.AsBP%20Key%20Object (Utilities|Casting|CastToBP_KeyObject (Variables|Default|GetInteract%20Actor)))) (Math|Rotator|MakeRotator (* _deltax 1e+01) (* _deltay 1e+01) 0.0) false false)))))))

(event EventBeginPlay
  (bind _mesh (Variables|Default|GetMesh))
  (Variables|Default|SetOriginalPosition (Transformation|GetWorldLocation _mesh))
  (Variables|Default|SetOriginalRotation (Transformation|GetWorldRotation _mesh)))

(fn ConstructionScript)