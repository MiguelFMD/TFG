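; GameSave is a Blueprint that holds saved dialogue data, grouped into narrative categories such as trauma, past, escape, search, clues and tasks.
; A single SaveDialogues event receives one value per category and copies each into its matching Saved variable.
; The graph only stores these values in memory, with no disk writing or load logic.
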(event Custom|SaveDialogues
  (params (DialogosTrauma :type Array%20of%20Names) (DialogosPasado :type Array%20of%20Names) (DialogosHuida :type Array%20of%20Names) (DialogosBusqueda :type Array%20of%20Names) (DialogosMolesto :type Array%20of%20Names) (DialogosEncuentra :type Array%20of%20Names) (DialogosPista :type Array%20of%20Names) (DialogosObjeto :type Array%20of%20Names) (DialogosInvestigando :type Array%20of%20Names) (DialogosEsperando :type Array%20of%20Names) (DialogosTarea :type Array%20of%20Names) (DialogosPregunta :type Array%20of%20Names) (DialogosHusmeando :type Array%20of%20Names))
  (Variables|Default|SetDialogosTraumaSaved DialogosTrauma)
  (Variables|Default|SetDialogosPasadoSaved DialogosPasado)
  (Variables|Default|SetDialogosHuidaSaved DialogosHuida)
  (Variables|Default|SetDialogosBusquedaSaved DialogosBusqueda)
  (Variables|Default|SetDialogosMolestoSaved DialogosMolesto)
  (Variables|Default|SetDialogosEncuentraSaved DialogosEncuentra)
  (Variables|Default|SetDialogosPistaSaved DialogosPista)
  (Variables|Default|SetDialogosObjetoSaved DialogosObjeto)
  (Variables|Default|SetDialogosInvestigandoSaved DialogosInvestigando)
  (Variables|Default|SetDialogosEsperandoSaved DialogosEsperando)
  (Variables|Default|SetDialogosTareaSaved DialogosTarea)
  (Variables|Default|SetDialogosPreguntaSaved DialogosPregunta)
  (Variables|Default|SetDialogosHusmeandoSaved DialogosHusmeando))