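; MenuCharacter is the character Blueprint that presents the main menu, with music and a fade-in.
; On BeginPlay it plays music, creates the MainMenu widget and switches input to UI-only with a visible cursor.
; One timeline alpha drives both the first-person camera's post-process Gain W and the widget's opacity.
; CloseMenu fades out the music and reverses that timeline to fade both back out.
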(event Custom|CloseMenu
  (Audio|Components|Audio|FadeOut (Variables|Default|GetStarter_Music01) 2.0 0.0 "Linear" :!class /Script/Engine.AudioComponent)
  (bind _alpha (Timeline|Timeline_0 Reverse)
    (:Update
      (Utilities|Struct|SetmembersinPostProcessSettings (Variables|/Script/Engine.CameraComponent|GetPostProcessSettings (Variables|MyCharacter|GetFirstPersonCamera)) (Math|Vector4|MakeVector4 1.0 1.0 1.0 _alpha))
      (Appearance|SetColorandOpacity (Variables|Default|GetMainMenu) (Math|Color|MakeColor 1.0 1.0 1.0 _alpha) :!class /Script/UMG.UserWidget))))

(event EventBeginPlay
  (bind _returnvalue (Game|GetPlayerController 0))
  (Audio|Components|Audio|Play (Variables|Default|GetStarter_Music01) 0.0)
  (bind _returnvalue_2 (UserInterface|CreateWidget "/Game/TFG/Widgets/MainMenu.MainMenu_C"))
  (bind _output_get (Variables|Default|SetMainMenu _returnvalue_2))
  (UserInterface|Viewport|AddtoViewport _output_get 0)
  (Variables|/Script/Engine.PlayerController|SetbShowMouseCursor _returnvalue true)
  (Input|SetInputModeUIOnly _returnvalue (Variables|Default|GetMainMenu) "DoNotLock")
  (bind _alpha (Timeline|Timeline_0 Play)
    (:Update
      (Utilities|Struct|SetmembersinPostProcessSettings (Variables|/Script/Engine.CameraComponent|GetPostProcessSettings (Variables|MyCharacter|GetFirstPersonCamera)) (Math|Vector4|MakeVector4 1.0 1.0 1.0 _alpha))
      (Appearance|SetColorandOpacity (Variables|Default|GetMainMenu) (Math|Color|MakeColor 1.0 1.0 1.0 _alpha) :!class /Script/UMG.UserWidget))))

(fn ConstructionScript)