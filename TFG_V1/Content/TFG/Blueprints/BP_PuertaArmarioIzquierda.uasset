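; Interactable left wardrobe door that swings open and closed when AbrirPuertaIzquierda is called.
; The event disables interaction and the custom-depth highlight, then plays a timeline from start or reverses it, depending on OpenedDoor.
; The timeline's Alpha drives the mesh's relative yaw, and its completion restores interaction and highlight.
; Tick derives OpenedDoor by checking Alpha against a threshold, so the flag follows the timeline position.
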(event Custom|AbrirPuertaIzquierda
  (Variables|Default|SetInteractable false)
  (Rendering|SetRenderCustomDepth (Variables|Character|GetMesh) false)
  (if (Variables|Default|GetOpenedDoor)
    (bind _alpha (Timeline|Timeline_0 PlayFromStart)
      (:Update
        (Transformation|SetRelativeRotation (Variables|Character|GetMesh) (Math|Rotator|MakeRotator 0.0 0.0 _alpha) false false))
      (:Finished
        (Variables|Default|SetInteractable true)
        (Rendering|SetRenderCustomDepth (Variables|Character|GetMesh) true)))
    (else
      (Timeline|Timeline_0 Reverse))))

(event EventTick
  (params (DeltaSeconds :type Float%20%28single-precision%29))
  (Variables|Default|SetOpenedDoor (> (stale Custom|AbrirPuertaIzquierda _alpha) -1.0)))

(fn ConstructionScript
  (|CallParentFunction))