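; BP_LockedDoor is a door that opens only when the player holds the matching key.
; OpenDoor searches the FirstPersonCharacter's Keys array for the door's DoorID and calls RotateDoor on a match.
; RotateDoor turns off interaction and the mesh's custom depth rendering, then plays the Rotate timeline, whose Alpha output drives the mesh's relative yaw directly.
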(event Custom|OpenDoor
  (params (Actor :type Actor%20Object%20Reference))
  (bind _asfirst_person_character (Utilities|Casting|CastToFirstPersonCharacter (Game|GetPlayerCharacter 0)))
  (bind _array_element (Utilities|Array|ForEachLoopwithBreak (Variables|/Game/TFG/Blueprints/FirstPersonCharacter.FirstPersonCharacter_C|GetKeys _asfirst_person_character) :!label _label)
    (:LoopBody
      (if (Utilities|Name|Equal(Name) _array_element (Variables|Default|GetDoorID))
        (CallFunction|RotateDoor)
        (goto _label Break)))))

(event Custom|RotateDoor
  (Variables|Default|SetInteractable false)
  (Rendering|SetRenderCustomDepth (Variables|Character|GetMesh) false)
  (bind _alpha (Timeline|Rotate PlayFromStart)
    (:Update
      (Transformation|SetRelativeRotation (Variables|Character|GetMesh) (Math|Rotator|MakeRotator 0.0 0.0 _alpha) false false))))

(fn ConstructionScript
  (|CallParentFunction))