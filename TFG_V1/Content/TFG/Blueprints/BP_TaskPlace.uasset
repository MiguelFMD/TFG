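; BP_TaskPlace is a trigger volume marking where a task item belongs.
; When an actor carrying this place's first tag enters the box while the first-person character holds an object, it sets that BP_TaskItem's InOriginPlace flag.
; Leaving clears the flag while holding, but that tag check tests the place itself rather than the leaving actor, so any BP_TaskItem qualifies.
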(event OnComponentBeginOverlap(Box)
  (params (OverlappedComponent :type Primitive%20Component%20Object%20Reference) (OtherActor :type Actor%20Object%20Reference) (OtherComp :type Primitive%20Component%20Object%20Reference) (OtherBodyIndex :type Integer) (bFromSweep :type Boolean) (SweepResult :type Hit%20Result%20Structure%20%28by%20ref%29))
  (bind _asfirst_person_character (Utilities|Casting|CastToFirstPersonCharacter (Game|GetPlayerCharacter 0)))
  (if (and (Actor|ActorHasTag OtherActor (Utilities|Array|Get(acopy) (Variables|Actor|GetTags))) (Variables|/Game/TFG/Blueprints/FirstPersonCharacter.FirstPersonCharacter_C|GetIs%20Holding%20Object? _asfirst_person_character))
    (bind _asbp_task_item (Utilities|Casting|CastToBP_TaskItem OtherActor))
    (Variables|/Game/TFG/Blueprints/BP_TaskItem.BP_TaskItem_C|SetInOriginPlace _asbp_task_item true)))

(event OnComponentEndOverlap(Box)
  (params (OverlappedComponent :type Primitive%20Component%20Object%20Reference) (OtherActor :type Actor%20Object%20Reference) (OtherComp :type Primitive%20Component%20Object%20Reference) (OtherBodyIndex :type Integer))
  (bind _asfirst_person_character (Utilities|Casting|CastToFirstPersonCharacter (Game|GetPlayerCharacter 0)))
  (if (and (Actor|ActorHasTag (Utilities|Array|Get(acopy) (Variables|Actor|GetTags))) (Variables|/Game/TFG/Blueprints/FirstPersonCharacter.FirstPersonCharacter_C|GetIs%20Holding%20Object? _asfirst_person_character))
    (bind _asbp_task_item (Utilities|Casting|CastToBP_TaskItem OtherActor))
    (Variables|/Game/TFG/Blueprints/BP_TaskItem.BP_TaskItem_C|SetInOriginPlace _asbp_task_item false)))

(fn ConstructionScript)