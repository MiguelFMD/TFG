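; Interactable world object that serves as the central dispatcher for player interactions such as doors, keys, hiding places and shortcuts.
; It flags itself as interactable on BeginPlay, and BeginInteract checks that flag on the target actor.
; A chain of casts then identifies the target's concrete class and calls its specific action, also covering check objects, drawers, wardrobe doors, collectible figures and locked doors.
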(event Custom|BeginInteract
  (params (InteractActor :type Actor%20Object%20Reference))
  (bind (_asbp_hiding_place _bsuccess) (Utilities|Casting|CastToBP_HidingPlace InteractActor))
  (bind (_asbp_locked_door _bsuccess_2) (Utilities|Casting|CastToBP_LockedDoor InteractActor))
  (bind (_asbp_new_key _bsuccess_3) (Utilities|Casting|CastToBP_NewKey InteractActor))
  (bind (_asbp_puerta_armario_izquierda _bsuccess_4) (Utilities|Casting|CastToBP_PuertaArmarioIzquierda InteractActor))
  (bind (_asbp_door _bsuccess_5) (Utilities|Casting|CastToBP_Door InteractActor))
  (bind (_asbp_cajon _bsuccess_6) (Utilities|Casting|CastToBP_Cajon InteractActor))
  (bind (_asbp_puerta_armario_derecha _bsuccess_7) (Utilities|Casting|CastToBP_PuertaArmarioDerecha InteractActor))
  (bind (_asbp_check_object _bsuccess_8) (Utilities|Casting|CastToBP_CheckObject InteractActor))
  (bind (_asbp_shortcut _bsuccess_9) (Utilities|Casting|CastToBP_Shortcut InteractActor))
  (bind (_asbp_figura _bsuccess_10) (Utilities|Casting|CastToBP_Figura InteractActor))
  (if (Variables|BP_InteractableObject_C|GetInteractable (.AsBP%20Interactable%20Object (Utilities|Casting|CastToBP_InteractableObject InteractActor)))
    (if _bsuccess_8
      (Default|BeginCheck _asbp_check_object InteractActor)
      (elif _bsuccess_9
        (Default|BeginShortCut _asbp_shortcut)
        (elif _bsuccess
          (Default|Hide _asbp_hiding_place)
          (elif _bsuccess_3
            (Default|CollectKey _asbp_new_key _asbp_new_key)
            (elif _bsuccess_5
              (Default|OpenDoor _asbp_door _asbp_door)
              (elif _bsuccess_6
                (Default|OpenDrawer _asbp_cajon _asbp_cajon)
                (elif _bsuccess_7
                  (Default|AbrirPuertaDerecha _asbp_puerta_armario_derecha)
                  (elif _bsuccess_4
                    (Default|AbrirPuertaIzquierda _asbp_puerta_armario_izquierda)
                    (elif _bsuccess_10
                      (Default|CollectFigura _asbp_figura _asbp_figura)
                      (elif _bsuccess_2
                        (Default|OpenDoor _asbp_locked_door _asbp_locked_door)))))))))))))

(event EventBeginPlay
  (Variables|Default|SetInteractable true))

(fn ConstructionScript)