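; BP_Figura is a collectible figure actor that records itself on the player when collected.
; Its CollectFigura event adds IDFigura to the FirstPersonCharacter's Figuras collection, then destroys the passed figure actor.
; A section marked development-only then fades the character's view and, after a short delay, opens the MainMenu level.
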(event Custom|CollectFigura
  (params (Figura :type BP%20Figura%20Object%20Reference))
  (bind _asfirst_person_character (Utilities|Casting|CastToFirstPersonCharacter (Game|GetPlayerCharacter 0)))
  (Utilities|Array|Add (Variables|/Game/TFG/Blueprints/FirstPersonCharacter.FirstPersonCharacter_C|GetFiguras _asfirst_person_character) (Variables|Default|GetIDFigura))
  (Actor|DestroyActor Figura)
  ;[0 1 0.2582] DEVELOPMENT ONLY
  (bind _asfirst_person_character_2 (Utilities|Casting|CastToFirstPersonCharacter (Game|GetPlayerCharacter 0)))
  (Default|Fade _asfirst_person_character_2 true)
  (Utilities|FlowControl|Delay 2.0)
  (Game|OpenLevel(byName) "MainMenu"))

(fn ConstructionScript
  (|CallParentFunction))