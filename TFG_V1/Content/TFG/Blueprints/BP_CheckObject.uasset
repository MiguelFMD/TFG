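; Inspectable object that the player pulls up to the view and rotates with the mouse.
; BeginCheck logs it in the character's ObjetosClave, adds any Respuestas table row matching its first tag, locks player input and moves the mesh to the character's VisualBox.
; While inspecting, Tick applies mouse-delta rotation and polls the FinishInteract keys.
; Finishing returns the mesh to its BeginPlay transform and restores input and HUD.
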(event Custom|BeginCheck
  (params (ActorToCheck :type Actor%20Object%20Reference))
  (bind _returnvalue (Game|GetPlayerCharacter 0))
  (bind _returnvalue_2 (Game|GetPlayerCharacter 0))
  (bind _asbp_interactable_object (Utilities|Casting|CastToBP_InteractableObject ActorToCheck))
  (bind _asfirst_person_character (Utilities|Casting|CastToFirstPersonCharacter _returnvalue))
  (bind _asfirst_person_character_2 (Utilities|Casting|CastToFirstPersonCharacter _returnvalue_2))
  (bind _mesh (Variables|/Game/TFG/Blueprints/BP_InteractableObject.BP_InteractableObject_C|GetMesh _asbp_interactable_object))
  (Utilities|Array|Add (Variables|/Game/TFG/Blueprints/FirstPersonCharacter.FirstPersonCharacter_C|GetObjetosClave _asfirst_person_character) (Variables|Default|GetName))
  (Default|DisplayInteractMessage (Variables|/Game/TFG/Blueprints/FirstPersonCharacter.FirstPersonCharacter_C|GetPlayerHUD _asfirst_person_character) 0 false)
  (CallFunction|CheckifResponse ActorToCheck)
  (Variables|/Game/TFG/Blueprints/FirstPersonCharacter.FirstPersonCharacter_C|SetPlayerInput _asfirst_person_character_2 false)
  (Variables|/Game/TFG/Blueprints/FirstPersonCharacter.FirstPersonCharacter_C|SetHusmeando _asfirst_person_character_2 true)
  (Variables|Default|SetActorToCheck ActorToCheck)
  (Physics|SetSimulatePhysics _mesh true)
  (Components|MoveComponentTo _mesh (Transformation|GetWorldLocation (Variables|/Game/TFG/Blueprints/FirstPersonCharacter.FirstPersonCharacter_C|GetVisualBox _asfirst_person_character_2)) "0, 0, 0" false false 0.2 false)
  (Default|DisplayObjectMessage (Variables|/Game/TFG/Blueprints/FirstPersonCharacter.FirstPersonCharacter_C|GetPlayerHUD (.AsFirst%20Person%20Character (Utilities|Casting|CastToFirstPersonCharacter (Game|GetPlayerCharacter 0)))) true))

(event Custom|CheckIfResponse
  (params (Actor :type Actor%20Object%20Reference))
  ;[1 1 1] Añadir pregunta
  (bind _returnvalue (Utilities|GetDataTableRow "/Game/TFG/Dialogs/Respuestas.Respuestas" (Utilities|Array|Get(acopy) (Variables|/Script/Engine.Actor|GetTags Actor)))
    (:then
      (bind _asfirst_person_character (Utilities|Casting|CastToFirstPersonCharacter (Game|GetPlayerCharacter 0)))
      (Utilities|Map|Add (Variables|/Game/TFG/Blueprints/FirstPersonCharacter.FirstPersonCharacter_C|GetRespuestas _asfirst_person_character) (Utilities|String|ToString(Text) (.Line (Utilities|Struct|BreakResponses_Struck _returnvalue))) (.Triggeredby (Utilities|Struct|BreakResponses_Struck _returnvalue))))))

(event EventTick
  (params (DeltaSeconds :type Float%20%28single-precision%29))
  (bind _returnvalue (Game|GetPlayerController 0))
  (bind _returnvalue_2 (Game|GetPlayerCharacter 0))
  (bind _returnvalue_3 (Game|GetPlayerController 0))
  (bind _actortocheck (Variables|Default|GetActorToCheck))
  (bind (_deltax _deltay) (Class|PlayerController|GetInputMouseDelta _returnvalue_3))
  (bind _asfirst_person_character (Utilities|Casting|CastToFirstPersonCharacter _returnvalue_2))
  (bind _asbp_interactable_object (Utilities|Casting|CastToBP_InteractableObject _actortocheck))
  (bind _mesh (Variables|/Game/TFG/Blueprints/BP_InteractableObject.BP_InteractableObject_C|GetMesh _asbp_interactable_object))
  (if (not (Variables|/Game/TFG/Blueprints/FirstPersonCharacter.FirstPersonCharacter_C|GetPlayerInput (.AsFirst%20Person%20Character (Utilities|Casting|CastToFirstPersonCharacter (Game|GetPlayerCharacter 0)))))
    (Utilities|IsValid (Variables|Default|GetActorToCheck)
      (:Is%20Valid
        (if (Game|Player|WasInputKeyJustPressed (Game|GetPlayerController 0) "AnyKey")
          (for _array_element (Class|InputSettings|GetActionMappingbyName (Class|InputSettings|GetInputSettings) "FinishInteract")
            (if (Game|Player|WasInputKeyJustPressed (Game|GetPlayerController 0) (.Key (Utilities|Struct|BreakInputActionKeyMapping _array_element)))
              (Components|MoveComponentTo _mesh (Variables|Default|GetOriginalPosition) (Variables|Default|GetOriginalRotation) false false 0.2 false)
              (Physics|SetSimulatePhysics _mesh false)
              (Input|SetInputModeGameOnly _returnvalue)
              (Input|EnableInput _returnvalue_2 _returnvalue)
              (Variables|/Game/TFG/Blueprints/FirstPersonCharacter.FirstPersonCharacter_C|SetPlayerInput _asfirst_person_character true)
              (Variables|/Game/TFG/Blueprints/FirstPersonCharacter.FirstPersonCharacter_C|SetHusmeando _asfirst_person_character false)
              (Default|DisplayObjectMessage (Variables|/Game/TFG/Blueprints/FirstPersonCharacter.FirstPersonCharacter_C|GetPlayerHUD (.AsFirst%20Person%20Character (Utilities|Casting|CastToFirstPersonCharacter (Game|GetPlayerCharacter 0)))) false)))
          (else
            (Transformation|AddLocalRotation (Variables|/Game/TFG/Blueprints/BP_InteractableObject.BP_InteractableObject_C|GetMesh (.AsBP%20Interactable%20Object (Utilities|Casting|CastToBP_InteractableObject (Variables|Default|GetActorToCheck)))) (Math|Rotator|MakeRotator (* _deltax 1e+01) (* _deltay 1e+01) 0.0) false false)))))))

(event EventBeginPlay
  (bind _mesh (Variables|Character|GetMesh))
  (Variables|Default|SetOriginalPosition (Transformation|GetWorldLocation _mesh))
  (Variables|Default|SetOriginalRotation (Transformation|GetWorldRotation _mesh)))

(fn ConstructionScript
  (|CallParentFunction))