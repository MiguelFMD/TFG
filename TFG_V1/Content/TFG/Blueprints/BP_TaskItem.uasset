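; BP_TaskItem is a world item tied to the game's task system that can be sent back to where it started.
; On BeginPlay it stores the actor's location and rotation as its origin.
; ReturnToOrigin moves the Mesh back to that stored transform, then calls AddItemToCurrentTask on MyGameInstance to register the item with the current task.
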(event Custom|ReturnToOrigin
  (Transformation|SetWorldLocationAndRotation (Variables|Default|GetMesh) (Variables|Default|GetOriginLocation) (Variables|Default|GetOriginRotation) false false)
  (Default|AddItemtoCurrentTask (.AsMy%20Game%20Instance (Utilities|Casting|CastToMyGameInstance (Game|GetGameInstance)))))

(event EventBeginPlay
  (Variables|Default|SetOriginLocation (Transformation|GetActorLocation))
  (Variables|Default|SetOriginRotation (Transformation|GetActorRotation)))

(fn ConstructionScript)