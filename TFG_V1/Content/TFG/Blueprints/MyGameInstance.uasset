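; Game instance that manages tag-based item tasks and reports their progress to an AI controller.
; BuildTask counts and enables items matching the task tag, shows the HUD message and highlights the task place via custom depth.
; AddItemToCurrentTask clears both on completion and sets AI blackboard flags for a finished task and for all tasks.
; PutItemsTaskInPlace moves every item to its TaskPlace with physics on and counts task places as the total.
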(event Custom|SetAI
  (params (AI :type AIC%20Loco%20Object%20Reference))
  (Variables|Default|SetAIC AI))

(fn BuildTask
  (params (TaskMessage :type Text) (Tag :type Name))
  (bind _output_get (Variables|Default|SetCurrentTask Tag))
  (bind _outactors (Actor|GetAllActorsOfClasswithTag "/Game/TFG/Blueprints/BP_TaskItem.BP_TaskItem_C" _output_get))
  (for _array_element _outactors
    (Variables|Default|SetItemsToFinishTask (+ (Variables|Default|GetItemsToFinishTask) 1))
    (Class|PrimitiveComponent|SetConstraintMode (Variables|/Game/TFG/Blueprints/BP_TaskItem.BP_TaskItem_C|GetMesh _array_element) "Default")
    (Variables|/Game/TFG/Blueprints/BP_TaskItem.BP_TaskItem_C|SetInteractable _array_element true))
  (Variables|Default|SetCurrentItems 0)
  (bind _asfirst_person_character (Utilities|Casting|CastToFirstPersonCharacter (Game|GetPlayerCharacter 0)))
  (Default|DisplayTaskMessage (Variables|/Game/TFG/Blueprints/FirstPersonCharacter.FirstPersonCharacter_C|GetPlayerHUD _asfirst_person_character) true TaskMessage)
  (bind _outactors_2 (Actor|GetAllActorsOfClasswithTag "/Game/TFG/Blueprints/BP_TaskPlace.BP_TaskPlace_C" (Variables|Default|GetCurrentTask)))
  (Rendering|SetRenderCustomDepth (Variables|/Game/TFG/Blueprints/BP_TaskPlace.BP_TaskPlace_C|GetMesh (Utilities|Array|Get(acopy) _outactors_2)) true))

(fn AddItemtoCurrentTask
  (bind _output_get (Variables|Default|SetCurrentItems (+ (Variables|Default|GetCurrentItems) 1)))
  (if (== _output_get (Variables|Default|GetItemsToFinishTask))
    (bind _outactors (Actor|GetAllActorsOfClasswithTag "/Game/TFG/Blueprints/BP_TaskPlace.BP_TaskPlace_C" (Variables|Default|GetCurrentTask)))
    (Rendering|SetRenderCustomDepth (Variables|/Game/TFG/Blueprints/BP_TaskPlace.BP_TaskPlace_C|GetMesh (Utilities|Array|Get(acopy) _outactors)) false)
    (Default|UpdateBlackBoardBool (Variables|Default|GetAIC) true "TareaAcabada")
    (bind _asfirst_person_character (Utilities|Casting|CastToFirstPersonCharacter (Game|GetPlayerCharacter 0)))
    (Default|DisplayTaskMessage (Variables|/Game/TFG/Blueprints/FirstPersonCharacter.FirstPersonCharacter_C|GetPlayerHUD _asfirst_person_character) false)
    (bind _output_get_2 (Variables|Default|SetTasksCompleted (+ (Variables|Default|GetTasksCompleted) 1)))
    (if (== _output_get_2 (Variables|Default|GetMaxNumberOfTasks))
      (Default|UpdateBlackBoardBool (Variables|Default|GetAIC) true "TasksCompleted"))))

(fn PutItemsTaskinPlace
  (bind _outactors (Actor|GetAllActorsOfClass "/Game/TFG/Blueprints/BP_TaskItem.BP_TaskItem_C"))
  (for _array_element _outactors
    (Physics|SetSimulatePhysics (Variables|/Game/TFG/Blueprints/BP_TaskItem.BP_TaskItem_C|GetMesh _array_element) true)
    (Variables|/Game/TFG/Blueprints/BP_TaskItem.BP_TaskItem_C|SetInOriginPlace _array_element false)
    (Transformation|SetWorldLocationAndRotation (Variables|/Game/TFG/Blueprints/BP_TaskItem.BP_TaskItem_C|GetMesh _array_element) (Transformation|GetWorldLocation (Variables|/Game/TFG/Blueprints/BP_TaskItem.BP_TaskItem_C|GetTaskPlace _array_element)) (Transformation|GetWorldRotation (Variables|/Game/TFG/Blueprints/BP_TaskItem.BP_TaskItem_C|GetTaskPlace _array_element)) false false))
  (bind _outactors_2 (Actor|GetAllActorsOfClass "/Game/TFG/Blueprints/BP_TaskPlace.BP_TaskPlace_C"))
  (for _array_element_2 _outactors_2
    (Variables|Default|SetMaxNumberOfTasks (+ (Variables|Default|GetMaxNumberOfTasks) 1))))