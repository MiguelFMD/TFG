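; BP_Door is a door that swings open through its OpenDoor event or when an IA_Loco character's capsule enters its Box trigger.
; OpenDoor calls RotateDoor, which clears Interactable, turns off the mesh's custom depth and plays a timeline that drives the mesh's relative yaw.
; When the rotation finishes, the NavModifier area class is set to NavArea_Obstacle; the file has no closing logic.
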(event OnComponentBeginOverlap(Box)
  (params (OverlappedComponent :type Primitive%20Component%20Object%20Reference) (OtherActor :type Actor%20Object%20Reference) (OtherComp :type Primitive%20Component%20Object%20Reference) (OtherBodyIndex :type Integer) (bFromSweep :type Boolean) (SweepResult :type Hit%20Result%20Structure%20%28by%20ref%29))
  (bind _asia_loco (Utilities|Casting|CastToIA_Loco OtherActor))
  (if (== (Variables|/Script/Engine.Character|GetCapsuleComponent _asia_loco) OtherComp)
    (CallFunction|OpenDoor)))

(event Custom|OpenDoor
  (params (Actor :type Actor%20Object%20Reference))
  (CallFunction|RotateDoor))

(event Custom|RotateDoor
  (Variables|Default|SetInteractable false)
  (Rendering|SetRenderCustomDepth (Variables|Character|GetMesh) false)
  (bind _alpha (Timeline|Rotate Play)
    (:Update
      (Transformation|SetRelativeRotation (Variables|Character|GetMesh) (Math|Rotator|MakeRotator 0.0 0.0 _alpha) false false))
    (:Finished
      (Class|NavModifierComponent|SetAreaClass (Variables|Collision|GetNavModifier) "/Script/NavigationSystem.NavArea_Obstacle"))))

(fn ConstructionScript
  (|CallParentFunction))