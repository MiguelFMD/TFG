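; Drawer actor that slides open or shut along its forward vector each time its OpenDrawer event fires.
; The Closed flag picks the direction, with the target set DistanceMove away from the current location.
; Separate Open and Close timelines lerp the whole actor there without sweeping.
; A Moving flag ignores new calls until a short delay after the slide finishes.
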(event Custom|OpenDrawer
  (params (Actor :type Actor%20Object%20Reference))
  (bind _returnvalue (Transformation|GetActorLocation))
  (bind _returnvalue_2 (Transformation|GetActorLocation))
  (if (not (Variables|Default|GetMoving))
    (Variables|Default|SetMoving true)
    (if (Variables|Default|GetClosed)
      (Variables|Default|SetTargetPoint (+ _returnvalue_2 (* (Transformation|GetActorForwardVector) (Variables|Default|GetDistanceMove))))
      (Variables|Default|SetCurrentLocation _returnvalue_2)
      (Variables|Default|SetClosed false)
      (bind _newtrack_0 (Timeline|Open PlayFromStart)
        (:Update
          (Transformation|SetActorLocation (Math|Vector|Lerp(Vector) (Variables|Default|GetCurrentLocation) (Variables|Default|GetTargetPoint) _newtrack_0) false false))
        (:Finished
          (Utilities|FlowControl|Delay 0.2)
          (Variables|Default|SetMoving false)))
      (else
        (Variables|Default|SetTargetPoint (+ _returnvalue (* (* (Transformation|GetActorForwardVector) -1.0) (Variables|Default|GetDistanceMove))))
        (Variables|Default|SetCurrentLocation _returnvalue)
        (Variables|Default|SetClosed true)
        (bind _newtrack_0_2 (Timeline|Close PlayFromStart)
          (:Update
            (Transformation|SetActorLocation (Math|Vector|Lerp(Vector) (Variables|Default|GetCurrentLocation) (Variables|Default|GetTargetPoint) _newtrack_0_2) false false))
          (:Finished
            (Utilities|FlowControl|Delay 0.2)
            (Variables|Default|SetMoving false)))))))

(fn ConstructionScript
  (|CallParentFunction))